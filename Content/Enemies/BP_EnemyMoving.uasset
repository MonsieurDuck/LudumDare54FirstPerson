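; BP_EnemyMoving is a goblin enemy that patrols back and forth until a player projectile kills it.
; Tick sweeps the mesh along its right vector at WalkingSpeed, unscaled by delta time, and overlapping a StaticMeshActor turns it 180 degrees.
; When a projectile's overlap ends, IsHit stops movement, body, skirt and armor meshes play a death animation, the game mode adds score, and the actor is destroyed after a delay.
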(event EventBeginPlay)

(event Collision|EventActorBeginOverlap
  (params (OtherActor :type Actor%20Object%20Reference))
  (if (not (Utilities|ClassIsChildOf (Utilities|GetClass OtherActor) "/Game/FirstPerson/Blueprints/BP_FirstPersonProjectile.BP_FirstPersonProjectile_C"))
    (Utilities|Casting|CastToStaticMeshActor OtherActor)
    (Transformation|SetWorldRotation (Variables|Default|GetSK_Goblin) (Math|Rotator|MakeRotator 0.0 0.0 (+ (.yaw (Transformation|GetWorldRotation (Variables|Default|GetSK_Goblin))) 1.8e+02)) false false)))

(event Collision|EventActorEndOverlap
  (params (OtherActor :type Actor%20Object%20Reference))
  (Utilities|Casting|CastToBP_FirstPersonProjectile OtherActor)
  (if (not (Variables|Default|GetIsHit?))
    (Variables|Default|SetIsHit? true)
    (CallFunction|PlayDeathAnimation)
    (bind _asbp_first_person_game_mode (Utilities|Casting|CastToBP_FirstPersonGameMode (Game|GetGameMode)))
    (Default|AddScore _asbp_first_person_game_mode)
    (Utilities|FlowControl|Delay 5.0)
    (Actor|DestroyActor)))

(event EventPlayDeathAnimation
  (Components|Animation|PlayAnimation (Variables|Default|GetSK_Goblin) "/Game/Goblin/Animation/Anim_Goblin_body_die_a.Anim_Goblin_body_die_a" false))

(event EventTick
  (params (DeltaSeconds :type Float%20%28single-precision%29))
  (if (not (Variables|Default|GetIsHit?))
    (Transformation|AddRelativeLocation (Variables|Default|GetSK_Goblin) (* (Math|Vector|GetRightVector (Variables|Default|GetSK_Goblin)) (Variables|Default|GetwalkingSpeed)) true false)))

(fn ConstructionScript
  (|CallParentFunction))