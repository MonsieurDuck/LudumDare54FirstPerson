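; Goblin enemy that plays a rage animation on spawn and dies when a first-person projectile hits it.
; Tick restarts a looping idle whenever the skeletal mesh stops playing an animation.
; The first projectile overlap sets a hit flag, plays the death animation, adds score through BP_FirstPersonGameMode, and destroys the actor after a short delay.
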(event Custom|PlayDeathAnimation
  (Components|Animation|PlayAnimation (Variables|Default|GetSK_Goblin) "/Game/Goblin/Animation/Anim_Goblin_body_die_b.Anim_Goblin_body_die_b" false))

(event EventBeginPlay
  (Components|Animation|PlayAnimation (Variables|Default|GetSK_Goblin) "/Game/Goblin/Animation/Anim_Goblin_body_rage.Anim_Goblin_body_rage" false))

(event EventTick
  (params (DeltaSeconds :type Float%20%28single-precision%29))
  (bind _sk_goblin (Variables|Default|GetSK_Goblin))
  (if (not (Audio|Components|Audio|IsPlaying _sk_goblin))
    (Components|Animation|PlayAnimation _sk_goblin "/Game/Goblin/Animation/Anim_Goblin_body_idle.Anim_Goblin_body_idle" true)))

(event Collision|EventActorBeginOverlap
  (params (OtherActor :type Actor%20Object%20Reference))
  (Utilities|Casting|CastToBP_FirstPersonProjectile OtherActor)
  (if (not (Variables|Default|GetIsHit?))
    (Variables|Default|SetIsHit? true)
    (CallFunction|PlayDeathAnimation)
    (bind _asbp_first_person_game_mode (Utilities|Casting|CastToBP_FirstPersonGameMode (Game|GetGameMode)))
    (Default|AddScore _asbp_first_person_game_mode)
    (Utilities|FlowControl|Delay 3.0)
    (Actor|DestroyActor)))

(fn ConstructionScript)