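; Enemy spawner that adds BP_Enemy pawns at random points inside its SpawnVolume, with difficulty rising over time.
; A looping four-second timer spawns one enemy only while the world's BP_Enemy count is within a cap that grows every ten seconds of time accumulated on Tick.
; Spawns use random X and Y at a fixed height, ignoring collision; a rotation toward the player is computed but left unconnected.
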(event Custom|spawn
  (bind _spawn_volume (Variables|Default|GetSpawn%20Volume))
  (bind _returnvalue (Transformation|GetWorldLocation _spawn_volume))
  (bind _returnvalue_2 (Components|Box|GetScaledBoxExtent _spawn_volume))
  (bind _returnvalue_3 (Math|Random|RandomPointinBoundingBox _returnvalue _returnvalue_2))
  (bind _outactors (Actor|GetAllActorsOfClass "/Game/Enemies/BP_Enemy.BP_Enemy_C"))
  (if (<= (Utilities|Array|Length _outactors) (Math|Float|Floor (/ (Variables|Default|GetTimer) 1e+01)))
    (AI|SpawnAIFromClass "/Game/Enemies/BP_Enemy.BP_Enemy_C" 0 (Math|Vector|MakeVector (.x _returnvalue_3) (.y _returnvalue_3) 5e+01) (Math|Rotator|MakeRotator 0.0 0.0 0.0) true 0)))

(event EventBeginPlay
  (Utilities|Time|SetTimerbyEvent (delegate Custom|spawn) 4.0 true))

(event EventTick
  (params (DeltaSeconds :type Float%20%28single-precision%29))
  (Variables|Default|Settimer (+ DeltaSeconds (Variables|Default|Gettimer))))

(fn ConstructionScript)