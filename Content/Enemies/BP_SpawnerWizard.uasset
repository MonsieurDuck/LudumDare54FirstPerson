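; BP_SpawnerWizard is a spawner that periodically adds wizard enemies inside its SpawnVolume.
; A looping timer attempts a spawn while the live wizard count is within a cap that grows with Tick-accumulated time, after an initial delay.
; Each attempt stores a random box point, spawns there at fixed height and plays a sound.
; The player-distance check rolls fresh random points rather than testing the stored location.
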(event Custom|spawn
  (bind _spawn_volume (Variables|Default|GetSpawn%20Volume))
  (bind _returnvalue (Transformation|GetWorldLocation _spawn_volume))
  (bind _returnvalue_2 (Components|Box|GetScaledBoxExtent _spawn_volume))
  (bind _returnvalue_3 (Math|Random|RandomPointinBoundingBox _returnvalue _returnvalue_2))
  (bind _outactors (Actor|GetAllActorsOfClass "/Game/Enemies/BP_EnemyWizard.BP_EnemyWizard_C"))
  (bind _output_get (Variables|Default|SetMax%20Enemies (Math|Float|Floor (/ (- (Variables|Default|GetTimer) 45.0) 3e+01))))
  (if (<= (Utilities|Array|Length _outactors) _output_get)
    (bind _output_get_2 (Variables|Default|Setspawn%20location (Math|Vector|MakeVector (.x _returnvalue_3) (.y _returnvalue_3) (.z _returnvalue_3))))
    (if (>= (Math|Vector|Distance(Vector) (Math|Vector|MakeVector (.x _returnvalue_3) (.y _returnvalue_3) (.z _returnvalue_3)) (Class|CharacterMovementComponent|GetLastUpdateLocation (Variables|/Script/Engine.Character|GetCharacterMovement (Game|GetPlayerCharacter 0)))) (Variables|Default|Getspawn%20radius))
      (bind _returnvalue_4 (AI|SpawnAIFromClass "/Game/Enemies/BP_EnemyWizard.BP_EnemyWizard_C" 0 (Math|Vector|MakeVector (.x _output_get_2) (.y _output_get_2) 5e+01) (Math|Rotator|MakeRotator 0.0 0.0 0.0) true 0))
      (Audio|PlaySoundatLocation "/Game/Sounds/SpawnWizard.SpawnWizard" (Transformation|GetActorLocation _returnvalue_4) "0, 0, 0" 1.3 1.0 1.3 "/Game/Sounds/goblinAttenuation.goblinAttenuation" 0 0 0))))

(event EventBeginPlay
  (Utilities|Time|SetTimerbyEvent (delegate Custom|spawn) 4.0 true))

(event EventTick
  (params (DeltaSeconds :type Float%20%28single-precision%29))
  (Variables|Default|Settimer (+ DeltaSeconds (Variables|Default|Gettimer))))

(fn ConstructionScript)