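; Goblin wizard enemy that turns to face the player and periodically charges and fires a projectile.
; A looping timer spawns the projectile, then Tick holds it at FireArrow, scales it with hold time and launches it after the attack animation starts.
; A player projectile hit sets IsHit, stopping attacks, disposing of the projectile, playing death, adding score and destroying the wizard after a delay.
; Animations play separately on each body, gear and staff mesh.
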(event Custom|Fire%20Projectile
  (if (not (Variables|Default|GetIsHit?))
    (bind _returnvalue (Game|SpawnActorfromClass "/Game/FirstPerson/Blueprints/BP_EnemyProjectile.BP_EnemyProjectile_C" (Transformation|GetWorldTransform (Variables|Default|GetFireArrow)) "Undefined" "MultiplyWithRoot" 0 0))
    (Variables|Default|SetBullet%20Is%20Charging true)))

(event Custom|IdleAnimation
  (Components|Animation|PlayAnimation (Variables|Default|GetSK_Goblin) "/Game/Goblin/Animation/Anim_Goblin_Wizard_attack_02.Anim_Goblin_Wizard_attack_02" false)
  (Components|Animation|PlayAnimation (Variables|Default|GetSK_Goblin_Wizard_Staff) "/Game/Goblin/Animation/Anim_Goblin_Wizard_Weapon_attack_02.Anim_Goblin_Wizard_Weapon_attack_02" false))

(event Custom|Attack%20Animation
  (Components|Animation|PlayAnimation (Variables|Default|GetSK_Goblin) "/Game/Goblin/Animation/Anim_Goblin_Wizard_attack_01.Anim_Goblin_Wizard_attack_01" false)
  (Components|Animation|PlayAnimation (Variables|Default|GetSK_Goblin_Wizard_Staff) "/Game/Goblin/Animation/Anim_Goblin_Wizard_attack_01.Anim_Goblin_Wizard_attack_01" false))

(event EventBeginPlay
  (bind _ishit_ (Variables|Default|GetIsHit?))
  (bind _returnvalue (not _ishit_))
  (if _returnvalue
    (CallFunction|FireProjectile)
    (if _returnvalue
      (Utilities|Time|SetTimerbyEvent (delegate Custom|Fire%20Projectile) 6.0 _returnvalue))))

(event EventTick
  (params (DeltaSeconds :type Float%20%28single-precision%29))
  (bind _sk_goblin (Variables|Default|GetSK_Goblin))
  (if (Variables|Default|GetIsHit?)
    (Default|DestroyProcess (stale Custom|Fire%20Projectile _returnvalue))
    (else
      (if (Audio|Components|Audio|IsPlaying (Variables|Default|GetSK_Goblin))
        _
        (else
          (CallFunction|IdleAnimation)))
      (Transformation|SetRelativeRotation _sk_goblin (Math|Rotator|MakeRotator 0.0 0.0 (- (.yaw (Math|Rotator|FindLookatRotation (Transformation|GetWorldLocation _sk_goblin) (Class|CharacterMovementComponent|GetLastUpdateLocation (Variables|/Script/Engine.Character|GetCharacterMovement (Game|GetPlayerCharacter 0))))) 9e+01)) false false)
      (if (Variables|Default|GetBullet%20Is%20Charging)
        (if (Variables|Default|GetIsHit?)
          (Actor|DestroyActor (stale Custom|Fire%20Projectile _returnvalue))
          (else
            (Transformation|SetActorTransform (stale Custom|Fire%20Projectile _returnvalue) (Transformation|GetWorldTransform (Variables|Default|GetFireArrow)))
            (if (>= (Variables|Default|GetBulletSize) 1.0)
              (Variables|Default|SetBulletSize 1.0)
              (else
                (Variables|Default|SetShoot%20Held%20Time (+ DeltaSeconds (Variables|Default|GetShoot%20Held%20Time)))
                (Variables|Default|SetBulletSize (* (Variables|Default|GetShoot%20Held%20Time) 0.1))))
            (if (not (Variables|Default|GetIsHit?))
              (Transformation|SetRelativeScale3D (Variables|/Game/FirstPerson/Blueprints/BP_EnemyProjectile.BP_EnemyProjectile_C|GetSphere (stale Custom|Fire%20Projectile _returnvalue)) (Math|Conversions|ToVector(Float) (Variables|Default|GetBulletSize)))
              (if (>= (Variables|Default|GetShoot%20Held%20Time) (Variables|Default|GetFireTime))
                (CallFunction|AttackAnimation)
                (Variables|Default|SetBullet%20Is%20Charging false)
                (Utilities|FlowControl|Delay 1.5)
                (Default|Fire (stale Custom|Fire%20Projectile _returnvalue) (Variables|Default|GetBulletSize))
                (Variables|Default|SetBulletSize 0.0)
                (Variables|Default|SetShoot%20Held%20Time 0.0)))))))))

(event Collision|EventActorBeginOverlap
  (params (OtherActor :type Actor%20Object%20Reference))
  (Utilities|Casting|CastToBP_FirstPersonProjectile OtherActor)
  (if (not (Variables|Default|GetIsHit?))
    (Variables|Default|SetIsHit? true)
    (CallFunction|PlayDeathAnimation)
    (bind _asbp_first_person_game_mode (Utilities|Casting|CastToBP_FirstPersonGameMode (Game|GetGameMode)))
    (Default|AddScore _asbp_first_person_game_mode)
    (Utilities|FlowControl|Delay 5.0)
    (Actor|DestroyActor)))

(event EventPlayDeathAnimation
  (Components|Animation|PlayAnimation (Variables|Default|GetSK_Goblin) "/Game/Goblin/Animation/Anim_Goblin_body_die_a.Anim_Goblin_body_die_a" false)
  (Components|Animation|PlayAnimation (Variables|Default|GetSK_Goblin_Wizard_Staff) "/Game/Goblin/Animation/Anim_Goblin_weapon_die_a.Anim_Goblin_weapon_die_a" false))

(fn ConstructionScript
  (|CallParentFunction))