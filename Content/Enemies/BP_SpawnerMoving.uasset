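; Spawner that adds moving enemies (BP_EnemyMoving) inside its SpawnVolume box as play time passes.
; A looping timer attempts spawns, gated by a live-enemy cap that starts after a delay and grows with Tick-accumulated time.
; Each enemy appears at a random XY and fixed height, facing one of two random yaws.
; An attenuated spawn sound plays at a separately randomized point in the box.
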(event Custom|spawn
  (bind _spawn_volume (Variables|Default|GetSpawn%20Volume))
  (bind _returnvalue (Transformation|GetWorldLocation _spawn_volume))
  (bind _returnvalue_2 (Components|Box|GetScaledBoxExtent _spawn_volume))
  (bind _returnvalue_3 (Math|Random|RandomPointinBoundingBox _returnvalue _returnvalue_2))
  (bind _outactors (Actor|GetAllActorsOfClass "/Game/Enemies/BP_EnemyMoving.BP_EnemyMoving_C"))
  (if (<= (Utilities|Array|Length _outactors) (Math|Float|Floor (/ (- (Variables|Default|GetTimer) 3e+01) 15.0)))
    (if (Math|Random|RandomBool)
      (Variables|Default|Setdirection 9e+01)
      (else
        (Variables|Default|Setdirection 0.0)))
    (AI|SpawnAIFromClass "/Game/Enemies/BP_EnemyMoving.BP_EnemyMoving_C" 0 (Math|Vector|MakeVector (.x _returnvalue_3) (.y _returnvalue_3) 5e+01) (Math|Rotator|MakeRotator 0.0 0.0 (Variables|Default|Getdirection)) true 0)
    (Audio|PlaySoundatLocation "/Game/Sounds/SpawnMoving.SpawnMoving" (Math|Vector|MakeVector (.x _returnvalue_3) (.y _returnvalue_3) (.z _returnvalue_3)) "0, 0, 0" 1.0 1.0 1.5 "/Game/Sounds/goblinAttenuation.goblinAttenuation" 0 0 0)))

(event EventBeginPlay
  (Utilities|Time|SetTimerbyEvent (delegate Custom|spawn) 4.0 true))

(event EventTick
  (params (DeltaSeconds :type Float%20%28single-precision%29))
  (Variables|Default|Settimer (+ DeltaSeconds (Variables|Default|Gettimer))))

(fn ConstructionScript)